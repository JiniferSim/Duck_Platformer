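; BP_Mama is the player-controlled mother duck character that leads ducklings, quacks and glides.
; Timelines animate the wings during jump input and the neck and legs during move input, while overlapping BP_Water raises walk speed.
; Each tick, ducklings inside the Sphere are told to follow, and that loop also restores normal gravity when grounded.
; Gliding zeroes vertical velocity mid-fall, then lowers gravity and boosts air control until release.
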(event Input|EnhancedActionEvents|EnhancedInputActionIA_Move
  (params (ActionValue :type Vector%202D%20Structure) (ElapsedSeconds :type Float%20%28double-precision%29) (TriggeredSeconds :type Float%20%28double-precision%29) (InputAction :type Input%20Action%20Object%20Reference :default "/Game/GameBase/Input/IA_Move.IA_Move"))
  ;[0.8073 0.6919 0.09118 0.5] Body and legs animation
  (:Started
    (bind (_direction _rotationvalue _legr _legl) (Timeline|SwingBody Play)
      (:Update
        (Transformation|SetRelativeRotation (Variables|Default|GetNeck) (Math|Rotator|MakeRotator 0.0 0.0 _rotationvalue) false false)
        (Transformation|SetRelativeRotation (Variables|Default|GetLeftLeg) (Math|Rotator|MakeRotator 0.0 _legl 0.0) false false)
        (Transformation|SetRelativeRotation (Variables|Default|GetRightLeg) (Math|Rotator|MakeRotator 0.0 _legr 0.0) false false))))
  (:Completed
    (Timeline|SwingBody Stop)))

(event Input|EnhancedActionEvents|EnhancedInputActionIA_Look
  (params (ActionValue :type Vector%202D%20Structure) (ElapsedSeconds :type Float%20%28double-precision%29) (TriggeredSeconds :type Float%20%28double-precision%29) (InputAction :type Input%20Action%20Object%20Reference :default "/Game/GameBase/Input/IA_Look.IA_Look"))
  ;[0.1158 0.03992 0.15 0.5] Camera movement
)

(event Input|EnhancedActionEvents|EnhancedInputActionIA_Jump
  (params (ActionValue :type Boolean) (ElapsedSeconds :type Float%20%28double-precision%29) (TriggeredSeconds :type Float%20%28double-precision%29) (InputAction :type Input%20Action%20Object%20Reference :default "/Game/GameBase/Input/IA_Jump.IA_Jump"))
  ;[0.06754 0.15 0.02305 0.5] Wings animation
  (:Started
    (bind (_direction _wingl _wingr) (Timeline|Wings Play)
      (:Update
        (Transformation|SetRelativeRotation (Variables|Default|GetWingL) (Math|Rotator|MakeRotator _wingl 0.0 0.0) false false)
        (Transformation|SetRelativeRotation (Variables|Default|GetWingR) (Math|Rotator|MakeRotator _wingr 0.0 0.0) false false))))
  (:Completed
    (Timeline|Wings Stop)))

(event Input|EnhancedActionEvents|EnhancedInputActionIA_Glide
  (params (ActionValue :type Vector%202D%20Structure) (ElapsedSeconds :type Float%20%28double-precision%29) (TriggeredSeconds :type Float%20%28double-precision%29) (InputAction :type Input%20Action%20Object%20Reference :default "/Game/GameBase/Input/IA_Glide.IA_Glide"))
  (bind _charactermovement (Variables|Character|GetCharacterMovement))
  (bind _charactermovement_2 (Variables|Character|GetCharacterMovement))
  ;[0.01539 0.08618 0.15 0.5] Gliding
  (:Started
    ;;[0.04544 0.7656 0.714 0.5] Glide
    (Utilities|FlowControl|DoOnce false :!label _label
      (:Completed
        (if (AI|Components|NavMovement|IsFalling _charactermovement)
          (Variables|/Script/Engine.MovementComponent|SetVelocity _charactermovement (Math|Vector|MakeVector (.x (Variables|/Script/Engine.MovementComponent|GetVelocity _charactermovement)) (.y (Variables|/Script/Engine.MovementComponent|GetVelocity _charactermovement)) 0.0))
          (Variables|/Script/Engine.CharacterMovementComponent|SetGravityScale _charactermovement 0.07)
          (Variables|/Script/Engine.CharacterMovementComponent|SetAirControl _charactermovement 0.7)
          (Utilities|FlowControl|Delay 0.2)
          (goto _label Reset)))))
  (:Completed
    ;;[0.04544 0.7656 0.714 0.5] Stop Glide
    (Variables|/Script/Engine.CharacterMovementComponent|SetGravityScale _charactermovement_2 1.0)
    (Variables|/Script/Engine.CharacterMovementComponent|SetAirControl _charactermovement_2 0.2)))

(event Input|EnhancedActionEvents|EnhancedInputActionIA_Quack
  (params (ActionValue :type Boolean) (ElapsedSeconds :type Float%20%28double-precision%29) (TriggeredSeconds :type Float%20%28double-precision%29) (InputAction :type Input%20Action%20Object%20Reference :default "/Game/GameBase/Input/IA_Quack.IA_Quack"))
  ;[0.15 0.007031 0.007031 0.5] Quacking
  (:Started
    (bind _returnvalue (AddComponent|AddAudioComponent false))
    (Variables|Default|SetMamaQuack _returnvalue))
  (:Completed
    (Audio|Components|Audio|Stop (Variables|Default|GetMamaQuack))))

(event EventTick
  (params (DeltaSeconds :type Float%20%28single-precision%29))
  (bind _charactermovement (Variables|Character|GetCharacterMovement))
  ;[0.15 0.121 0.004688 0.5] Setting Ducklin Follow Mama
  (for _array_element (Collision|GetOverlappingActors (Variables|Default|GetSphere) "/Game/Blueprints/BP-Ducklin.BP-Ducklin_C" :!class /Script/Engine.PrimitiveComponent)
    (bind _asbp_ducklin (Utilities|Casting|CastToBP-Ducklin _array_element))
    (Variables|/Game/Blueprints/BP-Ducklin.BP-Ducklin_C|SetFollowMama? _asbp_ducklin true)
    (Default|FollowMama _asbp_ducklin)
    ;[0.04544 0.7656 0.714 0.5] Gliding setting
    (if (AI|Components|NavMovement|IsMovingonGround _charactermovement)
      (Variables|/Script/Engine.CharacterMovementComponent|SetGravityScale _charactermovement 1.0)
      (Variables|/Script/Engine.CharacterMovementComponent|SetAirControl _charactermovement 0.2))))

(event Collision|EventActorBeginOverlap
  (params (OtherActor :type Actor%20Object%20Reference))
  ;[0.01341 0.2606 0.7217 0.5] Water speeding
  (Utilities|Casting|CastToBP_Water OtherActor)
  (Variables|/Script/Engine.CharacterMovementComponent|SetMaxWalkSpeed (Variables|Character|GetCharacterMovement) 4e+02))

(event Collision|EventActorEndOverlap
  (params (OtherActor :type Actor%20Object%20Reference))
  ;[0.01341 0.2606 0.7217 0.5] Water speeding
  (Utilities|Casting|CastToBP_Water OtherActor)
  (Variables|/Script/Engine.CharacterMovementComponent|SetMaxWalkSpeed (Variables|Character|GetCharacterMovement) 1.5e+02))

(fn ConstructionScript)