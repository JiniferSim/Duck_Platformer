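; BP_NestTutorial is a tutorial nest that detects ducklings brought home and signals when the goal is met.
; Each Tick it scans its Box overlaps, marks new ducklings collected, increments Mama's tally and zeroes their walk speed.
; It stops them following unless Mama is calling.
; Once the copied count equals one, it activates Niagara, flags all children home and plays a win sound once.
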(event Custom|All%20ducklin%20Safe
  ;[0.5365 0.109 0.109 0.5] When All children are collected Making VFX
  (if (== (Variables|Default|GetDuclingCount) 1)
    (Components|Activation|Activate (Variables|Default|GetNiagara) false)
    (Variables|Default|SetAllChildrenHome true)
    (Utilities|FlowControl|DoOnce false
      (:Completed
        (Audio|PlaySound2D "/Game/SFX/winner-game-sound-404167.winner-game-sound-404167" 0.7 1.0 0.0 0 0)))))

(event EventBeginPlay
  ;[0.00803 0.04307 0.15 0.5] Playing sound and Setting Mama
  (bind _asbp_mama (Utilities|Casting|CastToBP_Mama (Game|GetPlayerCharacter 0)))
  (Variables|Default|SetAs%20BP%20Mama _asbp_mama))

(event EventTick
  (params (DeltaSeconds :type Float%20%28single-precision%29))
  (bind _as_bp_mama (Variables|Default|GetAs%20BP%20Mama))
  ;[0.1768 0.6406 0.1846 0.5] Counting Ducklings
  (for _array_element (Collision|GetOverlappingActors (Variables|Default|GetBox) "/Game/Blueprints/BP-Ducklin.BP-Ducklin_C" :!class /Script/Engine.PrimitiveComponent)
    (bind _asbp_ducklin (Utilities|Casting|CastToBP-Ducklin _array_element))
    (if (not (Variables|/Game/Blueprints/BP-Ducklin.BP-Ducklin_C|Getcollected _asbp_ducklin))
      (bind _output_get (Variables|/Game/Blueprints/BP_Mama.BP_Mama_C|SetHow%20many%20ducklings _as_bp_mama (+ (Variables|/Game/Blueprints/BP_Mama.BP_Mama_C|GetHow%20many%20ducklings _as_bp_mama) 1)))
      (Variables|Default|SetDuclingCount _output_get)
      (Variables|/Game/Blueprints/BP-Ducklin.BP-Ducklin_C|Setcollected _asbp_ducklin true)
      (Variables|/Game/Blueprints/BP-Ducklin.BP-Ducklin_C|SetFollowMama? _asbp_ducklin false)
      (Variables|/Script/Engine.CharacterMovementComponent|SetMaxWalkSpeed (Variables|/Script/Engine.Character|GetCharacterMovement _asbp_ducklin) 0.0)
      (if (Variables|/Game/Blueprints/BP-Ducklin.BP-Ducklin_C|GetMamaCalling? _asbp_ducklin)
        (Variables|/Game/Blueprints/BP-Ducklin.BP-Ducklin_C|SetFollowMama? _asbp_ducklin true))))
  (CallFunction|AllDucklinSafe))

(fn ConstructionScript)