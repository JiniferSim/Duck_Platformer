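; BP_PlatformAppear is a platform that rises once enough pressure switches have activated it.
; Each Activation event increments a counter and compares it to the required switch count, stopping the Up timeline while short.
; Reaching the count passes a DoOnce and plays Up, whose track sets the box component's relative Z location.
; Debug strings print on activation and during the rise, and nothing decrements the counter.
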(event Custom|Activation
  (Development|PrintString "Activated")
  (Math|Integer|IncrementInt (Variables|Default|GetPressureSwitchActive)
    (:%20%20
      (if (>= (Variables|Default|GetPressureSwitchActive) (Variables|Default|GetPressureSwitchNeeded))
        (Utilities|FlowControl|DoOnce false
          (:Completed
            (bind _newtrack_0 (Timeline|Up Play)
              (:Update
                (Transformation|SetRelativeLocation (Variables|Default|GetBox_BA0B8AA3) (Math|Vector|MakeVector 0.0 0.0 _newtrack_0) false false)
                (Development|PrintString "Rising")))))
        (else
          (Timeline|Up Stop))))))

(fn ConstructionScript)